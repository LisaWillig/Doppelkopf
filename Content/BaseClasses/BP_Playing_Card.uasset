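; Base playing card actor that shows a card face and back on a mesh and can be dimmed when disabled.
; An integer picks the face from Cards, while a selector picks the CardBacks design, each becoming a dynamic material instance.
; Disabling tints the front through a vector parameter.
; The swap event rebuilds both material slots from the slot 0 material, despite its back/front naming, rather than rotating the mesh.
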(event EventSwapBackFront
  (CallFunction|SwapCardRotation))

(event EventCardDisable
  (params (bdisable :type Boolean))
  (Utilities|IsValid (Variables|Default|GetMID_CardFront)
    (:Is%20Valid
      (if bdisable
        (Rendering|Material|SetVectorParameterValue (Variables|Default|GetMID_CardFront) "FCol_DisableCard" "(R=0.177083,G=0.177083,B=0.177083,A=0.650000)" :!class /Script/Engine.MaterialInstanceDynamic)
        (else
          (Rendering|Material|SetVectorParameterValue (Variables|Default|GetMID_CardFront) "FCol_DisableCard" "(R=1.000000,G=1.000000,B=1.000000,A=0.000000)" :!class /Script/Engine.MaterialInstanceDynamic))))))

(event EventSetCardFromtInt
  (params (value :type Integer))
  (CallFunction|SetValuebyInteger value))

(fn ConstructionScript)

(fn SetValuebyInteger
  (params (CardByInteger :type Integer))
  (bind _returnvalue (Rendering|Material|CreateDynamicMaterialInstance (Variables|Default|GetCardMesh) 0 (Utilities|Array|Get(acopy) (Variables|Default|GetCards) CardByInteger) "None" :!class /Script/Engine.PrimitiveComponent))
  (Variables|Default|SetMID_CardFront _returnvalue)
  (bind _returnvalue_2 (Rendering|Material|CreateDynamicMaterialInstance (Variables|Default|GetCardMesh) 1 (Utilities|Array|Get(acopy) (Variables|Default|GetCardBacks) (Utilities|Select :Index "NewEnumerator1" :NewEnumerator1 0 :NewEnumerator2 1 :NewEnumerator3 2 :NewEnumerator4 3 :NewEnumerator5 4 :NewEnumerator6 5 :NewEnumerator7 6 :NewEnumerator8 7 :NewEnumerator9 8 :NewEnumerator10 9 :NewEnumerator11 10 :NewEnumerator12 11 :NewEnumerator13 12 :NewEnumerator14 13 :NewEnumerator15 14 :NewEnumerator16 15 :NewEnumerator17 16 :NewEnumerator18 17 :NewEnumerator19 18 :NewEnumerator20 19 :NewEnumerator21 20 :NewEnumerator22 21 :NewEnumerator23 22 :NewEnumerator24 23 :NewEnumerator25 24 :NewEnumerator37 25 :NewEnumerator38 26 :NewEnumerator39 27 :NewEnumerator40 28 :NewEnumerator41 29 :NewEnumerator42 30 :NewEnumerator43 31 :NewEnumerator44 32 :NewEnumerator45 33 :NewEnumerator46 34 :NewEnumerator47 35 :NewEnumerator48 36)) "None" :!class /Script/Engine.PrimitiveComponent))
  (Variables|Default|SetMID_CardBack _returnvalue_2)
  (return))

(fn SwapCardRotation
  (bind _cardmesh (Variables|Default|GetCardMesh))
  (bind _returnvalue (Rendering|Material|GetMaterials _cardmesh))
  (bind _returnvalue_2 (Rendering|Material|CreateDynamicMaterialInstance (Variables|Default|GetCardMesh) 1 (Utilities|Array|Get(acopy) _returnvalue) "None" :!class /Script/Engine.PrimitiveComponent))
  (Variables|Default|SetMID_CardBack _returnvalue_2)
  (bind _returnvalue_3 (Rendering|Material|CreateDynamicMaterialInstance (Variables|Default|GetCardMesh) 0 (Utilities|Array|Get(acopy) _returnvalue) "None" :!class /Script/Engine.PrimitiveComponent))
  (Variables|Default|SetMID_CardFront _returnvalue_3))