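; Player controller for a Doppelkopf card game that shows the HUD during the local player's turn.
; It creates a WBP_HUD widget on BeginPlay, then polls the player state's MyTurn flag every tick to add it to or remove it from the viewport.
; Pressing K asks BP_DoppelkopfMode to spawn an AI.
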(event EventBeginPlay
  (bind _returnvalue (UserInterface|CreateWidget "/Game/MenuSystem/WBP_HUD.WBP_HUD_C" (Game|GetPlayerController 0)))
  (Variables|Default|SetHUD _returnvalue))

(event EventTick
  (params (DeltaSeconds :type Float%20%28single-precision%29))
  (bind _asdoppelkopf_player_state (Utilities|Casting|CastToDoppelkopfPlayerState (Variables|Default|GetPlayerState)))
  (if (Variables|/Script/Doppelkopf.DoppelkopfPlayerState|GetmyTurn _asdoppelkopf_player_state)
    (Utilities|IsValid (Variables|Default|GetHUD)
      (:Is%20Valid
        (UserInterface|Viewport|AddtoViewport (Variables|Default|GetHUD) 0)))
    (else
      (Utilities|IsValid (Variables|Default|GetHUD)
        (:Is%20Valid
          (Widget|RemovefromParent (Variables|Default|GetHUD)))))))

(event Input|KeyboardEvents|K
  (params (Key :type Key%20Structure :default "None"))
  (:Pressed
    (bind _asbp_doppelkopf_mode (Utilities|Casting|CastToBP_DoppelkopfMode (Game|GetGameMode)))
    (Default|SpawnAI _asbp_doppelkopf_mode)))

(fn ConstructionScript)